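; BP_Upgrade is a purchasable upgrade button that levels up its associated room.
; Its BuyButton override runs the parent purchase logic, calls UpgradeRoom on the associated room, then copies that room's BuyCost into its own cost.
; It destroys itself once the room's level index reaches 2 or higher.
; The event graph is unused, and the construction script only calls the parent.
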(event EventBeginPlay)

(event Collision|EventActorBeginOverlap
  (params (OtherActor :type Actor%20Object%20Reference)))

(event EventTick
  (params (DeltaSeconds :type Float%20%28single-precision%29)))

(fn ConstructionScript
  (|CallParentFunction))

(fn BuyButton
  (bind _assocroom (Variables|Default|GetAssocRoom))
  (|CallParentFunction)
  (Default|UpgradeRoom _assocroom)
  (bind _asbp_parent_room (Utilities|Casting|CastToBP_ParentRoom _assocroom))
  (Variables|Default|SetCost (Variables|/Game/Blueprints/RoomsBlueprints/BP_ParentRoom.BP_ParentRoom_C|GetBuyCost _asbp_parent_room))
  (if (>= (Variables|/Game/Blueprints/RoomsBlueprints/BP_ParentRoom.BP_ParentRoom_C|GetIndexForLevels _asbp_parent_room) 2)
    (Actor|DestroyActor)))