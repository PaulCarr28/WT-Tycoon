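; BP_AddButton is a clickable purchase button actor for a tycoon game that spends the player's money.
; BeginPlay creates its own BP_MoneyWidget, adds it to the viewport and keeps the reference.
; On click, Purchase checks GM_Tycoon's CurrentMoney against Cost, sets IsPurchased and returns the remaining balance.
; The click handler rechecks affordability, writes that balance to the game mode, destroys the button and refreshes the widget.
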(event EventBeginPlay
  ;[1 1 1] Create Widget In add Button Bp because the return value is needed for casting
  (bind _returnvalue (UserInterface|CreateWidget "/Game/Blueprints/BP_MoneyWidget.BP_MoneyWidget_C"))
  (UserInterface|Viewport|AddtoViewport _returnvalue 0))

(event MouseInput|EventActorOnClicked
  (params (ButtonPressed :type Key%20Structure :default "None"))
  ;[1 1 1] Purchased Removes Money From Cost
  (bind _money (CallFunction|Purchase))
  (bind _asgm_tycoon (Utilities|Casting|CastToGM_Tycoon (Game|GetGameMode)))
  (if (>= (Variables|/Game/Core/GM_Tycoon.GM_Tycoon_C|GetCurrentMoney _asgm_tycoon) (Variables|Default|GetCost))
    (if (Variables|Default|GetIsPurchased?)
      (Variables|/Game/Core/GM_Tycoon.GM_Tycoon_C|SetCurrentMoney _asgm_tycoon _money)
      (Actor|DestroyActor)
      (Default|UpdateMoney (stale EventBeginPlay _returnvalue)))))

(fn ConstructionScript)

(fn Purchase
  ;[1 1 1] Purchase
  (bind _asgm_tycoon (Utilities|Casting|CastToGM_Tycoon (Game|GetGameMode)))
  (if (>= (Variables|/Game/Core/GM_Tycoon.GM_Tycoon_C|GetCurrentMoney _asgm_tycoon) (Variables|Default|GetCost))
    (Variables|Default|SetIsPurchased? true)
    (return (- (Variables|/Game/Core/GM_Tycoon.GM_Tycoon_C|GetCurrentMoney _asgm_tycoon) (Variables|Default|GetCost)))))