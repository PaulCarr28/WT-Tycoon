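; BP_Add is a purchasable placeholder actor that becomes a room when bought.
; Its BuyButton override calls the parent logic, spawns AssocBlueprint and a BP_Upgrade actor at its own transform, then destroys itself.
; The new BP_Upgrade receives the spawned actor as its AssocRoom, so the add spot turns into an upgrade point for that room.
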(event EventBeginPlay
  (|CallParentFunction) ; This node is disabled and will not be called.\nDrag off pins to build functionality.
)

(event Collision|EventActorBeginOverlap
  (params (OtherActor :type Actor%20Object%20Reference)))

(event EventTick
  (params (DeltaSeconds :type Float%20%28single-precision%29)))

(fn ConstructionScript
  (|CallParentFunction))

(fn BuyButton
  (bind _returnvalue (Transformation|GetActorTransform))
  (|CallParentFunction)
  (bind _returnvalue_2 (Game|SpawnActorfromClass (Variables|Default|GetAssocBlueprint) _returnvalue "Undefined" "MultiplyWithRoot" 0 0))
  (bind _returnvalue_3 (Game|SpawnActorfromClass "/Game/Blueprints/BP_Upgrade.BP_Upgrade_C" _returnvalue "Undefined" "MultiplyWithRoot" 0 0))
  (Variables|/Game/Blueprints/BP_Upgrade.BP_Upgrade_C|SetAssocRoom _returnvalue_3 _returnvalue_2)
  (Actor|DestroyActor))