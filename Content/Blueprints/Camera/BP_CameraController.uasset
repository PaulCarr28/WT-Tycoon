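; Camera controller actor that pans across the world horizontally while the right mouse button is held and dragged.
; Tick maps the viewport mouse delta, with axes swapped and one negated, to a world XY offset, then prints the location.
; A FlipFlop alternates that movement with a bounds check on successive held ticks.
; Leaving the fixed box around world origin snaps the actor back to its BeginPlay location.
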(event EventBeginPlay
  (Variables|Default|SetActorOrigin (Transformation|GetActorLocation)))

(event EventTick
  (params (DeltaSeconds :type Float%20%28single-precision%29))
  (bind _returnvalue (Class|WidgetLayoutLibrary|GetMousePositiononViewport))
  (if (Game|Player|IsInputKeyDown (Game|GetPlayerController 0) "RightMouseButton")
    (Utilities|FlowControl|FlipFlop
      (:A
        (if (not (Math|Geometry|IsPointinBox (Transformation|GetActorLocation) "0, 0, 0" "7260.000000,5630.000000,1181.000000"))
          (Transformation|SetActorLocation (Variables|Default|GetActorOrigin) false false)))
      (:B
        (Variables|Default|SetNewCamLoc _returnvalue)
        (Transformation|AddActorWorldOffset (Math|Vector|MakeVector (.y (- (Variables|Default|GetNewCamLoc) (Variables|Default|GetCameraPrevLoc))) (* (.x (- (Variables|Default|GetNewCamLoc) (Variables|Default|GetCameraPrevLoc))) -1.0) 0.0))
        (Variables|Default|SetCameraPrevLoc (Variables|Default|GetNewCamLoc))
        (Development|PrintString (Utilities|String|ToString(Vector) (Transformation|GetActorLocation)))))))

(event Input|ActionEvents|InputActionRightMouseDrag
  (params (Key :type Key%20Structure :default "None"))
  (:Pressed
    (bind _returnvalue (Class|WidgetLayoutLibrary|GetMousePositiononViewport))
    (Variables|Default|SetCameraPrevLoc _returnvalue)))

(fn ConstructionScript)