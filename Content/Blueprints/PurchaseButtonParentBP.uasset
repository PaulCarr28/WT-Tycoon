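; Parent actor Blueprint for clickable purchase buttons in a tycoon game, charging the player for an associated room.
; BeginPlay reads the cost from the associated Blueprint's class defaults, and Tick rewrites the cost text every frame.
; Clicking runs BuyButton, which deducts the cost from GM_Tycoon's current money when affordable and returns a purchased flag, otherwise printing a failure message.
; No room spawning happens here.
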(event EventBeginPlay
  (bind _assocblueprint (Variables|Default|GetAssocBlueprint))
  (bind _buycost (Utilities|GetClassDefaults _assocblueprint))
  ;[1 1 1] Sets the cost of the button to the cost of the room
  (Variables|Default|SetCost _buycost)
  (Rendering|Components|TextRender|SetText (Variables|Default|GetCostText) (Utilities|Text|ToText(String) (Utilities|String|ToString(Integer) _buycost))))

(event EventTick
  (params (DeltaSeconds :type Float%20%28single-precision%29))
  (Rendering|Components|TextRender|SetText (Variables|Default|GetCostText) (Utilities|Text|ToText(String) (Utilities|String|ToString(Integer) (Variables|Default|GetCost)))))

(event MouseInput|EventActorOnClicked
  (params (ButtonPressed :type Key%20Structure :default "None"))
  ;[1 1 1] Purchased Removes Money From Cost
  (CallFunction|BuyButton))

(fn ConstructionScript)

(fn BuyButton
  ;[1 1 1] Purchase
  (bind _asgm_tycoon (Utilities|Casting|CastToGM_Tycoon (Game|GetGameMode)))
  (if (>= (Variables|/Game/Core/GM_Tycoon.GM_Tycoon_C|GetCurrentMoney _asgm_tycoon) (Variables|Default|GetCost))
    (Variables|Default|SetIsPurchased? true)
    (Variables|/Game/Core/GM_Tycoon.GM_Tycoon_C|SetCurrentMoney _asgm_tycoon (- (Variables|/Game/Core/GM_Tycoon.GM_Tycoon_C|GetCurrentMoney _asgm_tycoon) (Variables|Default|GetCost)))
    (else
      (Development|PrintString "Failed to buy!")
      (Variables|Default|SetIsPurchased? false)))
  (return (Variables|Default|GetIsPurchased?)))