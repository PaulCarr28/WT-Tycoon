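; GM_Tycoon is the game mode for a tycoon game, holding the money and year state.
; On BeginPlay it sets the starting money and adds the BP_MoneyWidget to the viewport.
; A looping timer advances the year at a fixed interval, and reaching the final year opens the EndScreen level.
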(event Custom|YearUp
  ;[1 1 1] Add Year Every 20 Sec
  (Variables|Default|SetYear (+ (Variables|Default|GetYear) 1))
  (if (== (Variables|Default|GetYear) 50)
    (Game|OpenLevel(byObjectReference) "/Game/Maps/EndScreen.EndScreen")))

(event EventBeginPlay
  ;[1 1 1] Add Money To Viewport
  (Variables|Default|SetCurrentMoney 2)
  (Utilities|Time|SetTimerbyEvent (delegate Custom|YearUp) 2e+01 true)
  (bind _returnvalue (UserInterface|CreateWidget "/Game/Blueprints/BP_MoneyWidget.BP_MoneyWidget_C"))
  (bind _output_get (Variables|Default|SetWidgetRef _returnvalue))
  (UserInterface|Viewport|AddtoViewport _output_get 0))

(fn ConstructionScript)